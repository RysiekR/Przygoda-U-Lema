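; BP_PuzzleTrigger is an energy-driven trigger that activates a set of puzzle pieces once fully charged.
; It forwards Charge and Drain events to its Energy component and binds to that component's full-charge event on BeginPlay.
; On full charge it sends an Activate message to every entry in PuzzlePieces and prints a debug string.
; A getter exposes the Energy component to other objects.
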(event Custom|FullCharge
  (for _array_element (Variables|Default|GetPuzzlePieces)
    (Class|BPIPuzzlePieces|Activate(Message) _array_element))
  (Development|PrintString "Done all activates on every piece"))

(event EventBeginPlay
  (EventDispatchers|BindEventtoFullCharge (Variables|Default|GetEnergy) (EventDispatchers|CreateEvent :!event Custom|FullCharge)))

(event EventCharge
  (params (Amount :type Float%20%28double-precision%29))
  (Default|CallChargeEnergy (Variables|Default|GetEnergy) Amount))

(event EventDrain
  (params (Amount :type Float%20%28double-precision%29))
  (Default|CallDrainEnergy (Variables|Default|GetEnergy) Amount))

(fn ConstructionScript)

(fn GetEnergyComponent
  (return (Variables|Default|GetEnergy)))