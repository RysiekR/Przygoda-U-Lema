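; BP_StickyHookFinal is a grappling hook projectile that sticks to surfaces tagged WallToJump and pulls its firer toward them.
; On spawn it registers itself with the first-person instigator's GrapplingLogic to start a wall grapple.
; On the first collision with a tagged wall it sets a sticking flag, tells the instigator to start the pull and halts its projectile movement.
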(event OnComponentHit(CollisionComponent)
  (params (HitComponent :type Primitive%20Component%20Object%20Reference) (OtherActor :type Actor%20Object%20Reference) (OtherComp :type Primitive%20Component%20Object%20Reference) (NormalImpulse :type Vector :default "0, 0, 0") (Hit :type Hit%20Result%20Structure%20%28by%20ref%29))
  (if (Actor|ActorHasTag OtherActor "WallToJump")
    (if (not (Variables|Default|GetIsSticking?))
      (Variables|Default|SetIsSticking? true)
      (Default|CallStartGrapplePulltoWall (Variables|Default|GetInstigatorFirstPerson))
      (Components|Movement|StopMovementImmediately (Variables|Default|GetProjectileMovement)))))

(event EventBeginPlay
  (Default|StartGrappletoWall (Variables|/Game/LemGame/Player/FirstPerson/Blueprints/BP_FirstPersonCharacter.BP_FirstPersonCharacter_C|GetGrapplingLogic (Variables|Default|GetInstigatorFirstPerson)) self))

(fn ConstructionScript)