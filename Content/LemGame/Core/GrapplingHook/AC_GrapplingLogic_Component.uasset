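; Actor component that runs the first-person character's grappling hook, with separate wall and item grapples.
; It binds to character events to start, pull and stop each grapple, toggling cables and destroying hook actors.
; Tick pins cable ends to the hooks and applies force, flying the player toward walls with sideways input steering or dragging items toward the player.
; Attaching and pulling call the character's Drain.
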(event Custom|StopGrappleToWall
  ;[1 1 1] Stop Grapple To Wall
  (if (Variables|Default|GetIsGrapplingWall?)
    (Variables|Default|SetIsGrapplingWall? false)
    (Variables|Default|SetIsPullingToWall? false)
    (Pawn|Components|CharacterMovement|SetMovementMode (Variables|/Script/Engine.Character|GetCharacterMovement (Variables|Default|GetFirstPlayerCharacter)) "MOVE_Falling" 0)
    (Rendering|SetVisibility (Variables|/Game/LemGame/Player/FirstPerson/Blueprints/BP_FirstPersonCharacter.BP_FirstPersonCharacter_C|GetCableToWall (Variables|Default|GetFirstPlayerCharacter)) false false)
    (Actor|DestroyActor (Variables|Default|GetWallHook))
    (else
      (Development|PrintString "stop grapple wall"))))

(event Custom|StartGrappleItem
  (params (NewParam :type BP%20Light%20Hook%20Final%20Object%20Reference))
  ;[1 1 1] Start Grapple Item
  (Utilities|IsValid NewParam
    (:Is%20Valid
      (Development|PrintString "item")
      (if (Variables|Default|GetCanGrappleItem?)
        (if (not (Variables|Default|GetIsPullingItem?))
          (Variables|Default|SetItemHook NewParam)
          (Variables|Default|SetIsGrapplingItem? true)
          (Rendering|SetVisibility (Variables|/Game/LemGame/Player/FirstPerson/Blueprints/BP_FirstPersonCharacter.BP_FirstPersonCharacter_C|GetCableToItem (Variables|Default|GetFirstPlayerCharacter)) true false)
          (Default|Drain (Variables|Default|GetFirstPlayerCharacter) 0.5))))
    (:Is%20Not%20Valid
      (Development|PrintString "invalid grappleitem"))))

(event Custom|StopGrappleItem
  ;[1 1 1] Stop Grapple Item
  (if (Variables|Default|GetIsGrapplingItem?)
    (Variables|Default|SetIsGrapplingItem? false)
    (Variables|Default|SetIsPullingItem? false)
    (Rendering|SetVisibility (Variables|/Game/LemGame/Player/FirstPerson/Blueprints/BP_FirstPersonCharacter.BP_FirstPersonCharacter_C|GetCableToItem (Variables|Default|GetFirstPlayerCharacter)) false false)
    (Actor|DestroyActor (Variables|Default|GetItemHook))
    (else
      (Development|PrintString "stop grapple item"))))

(event Custom|StartGrappleToWall
  (params (GrapplePoint :type BP%20Sticky%20Hook%20Final%20Object%20Reference))
  ;[1 1 1] Start Grapple To Wall
  (Utilities|IsValid GrapplePoint
    (:Is%20Valid
      (Development|PrintString "sticky")
      (if (Variables|Default|GetCanGrappleToWall?)
        (if (not (Variables|Default|GetIsGrapplingWall?))
          (Variables|Default|SetWallHook GrapplePoint)
          (Variables|Default|SetIsGrapplingWall? true)
          (Rendering|SetVisibility (Variables|/Game/LemGame/Player/FirstPerson/Blueprints/BP_FirstPersonCharacter.BP_FirstPersonCharacter_C|GetCableToWall (Variables|Default|GetFirstPlayerCharacter)) true false)
          (Default|Drain (Variables|Default|GetFirstPlayerCharacter) 0.5))))
    (:Is%20Not%20Valid
      (Development|PrintString "invalid grapple wall"))))

(event Custom|StartGrapplePullToWall
  ;[1 1 1] Start Pulling To Wall
  (if (Variables|Default|GetCanGrappleToWall?)
    (if (Variables|Default|GetIsGrapplingWall?)
      (Variables|Default|SetIsPullingToWall? true)
      (Pawn|Components|CharacterMovement|SetMovementMode (Variables|/Script/Engine.Character|GetCharacterMovement (Variables|Default|GetFirstPlayerCharacter)) "MOVE_Flying" 0))))

(event Custom|StartGrapplePullItem
  ;[1 1 1] Start Pulling Item
  (if (Variables|Default|GetCanGrappleItem?)
    (if (Variables|Default|GetIsGrapplingItem?)
      (Variables|Default|SetIsPullingItem? true))))

(event EventBeginPlay
  ;[1 1 1] Hooking events From FirstPlayerCharacter
  (bind _asbp_first_person_character (Utilities|Casting|CastToBP_FirstPersonCharacter (Components|GetOwner)))
  (Variables|Default|SetFirstPlayerCharacter _asbp_first_person_character)
  (EventDispatchers|BindEventtoStartGrappletoWall (Variables|Default|GetFirstPlayerCharacter) (EventDispatchers|CreateEvent :!event Custom|StartGrappleToWall))
  (EventDispatchers|BindEventtoStopGrappletoWall (Variables|Default|GetFirstPlayerCharacter) (EventDispatchers|CreateEvent :!event Custom|StopGrappleToWall))
  (EventDispatchers|BindEventtoStartGrapplePulltoWall (Variables|Default|GetFirstPlayerCharacter) (EventDispatchers|CreateEvent :!event Custom|StartGrapplePullToWall))
  (EventDispatchers|BindEventtoStartGrapplePullItem (Variables|Default|GetFirstPlayerCharacter) (EventDispatchers|CreateEvent :!event Custom|StartGrapplePullItem))
  (EventDispatchers|BindEventtoStopGrappleItem (Variables|Default|GetFirstPlayerCharacter) (EventDispatchers|CreateEvent :!event Custom|StopGrappleItem))
  (EventDispatchers|BindEventtoStartGrappleItem (Variables|Default|GetFirstPlayerCharacter) (EventDispatchers|CreateEvent :!event Custom|StartGrappleItem)))

(event EventTick
  (params (DeltaSeconds :type Float%20%28single-precision%29))
  (Utilities|FlowControl|Sequence
    (:then_0
      (if (Variables|Default|GetIsGrapplingWall?)
        ;[1 1 1] Setting End Point of The Wall Hook
        (bind _wallhook (Variables|Default|GetWallHook)
          (:then
            (Variables|Default|SetWallHookLocation (Transformation|GetActorLocation _wallhook))
            (Variables|/Script/CableComponent.CableComponent|SetEndLocation (Variables|/Game/LemGame/Player/FirstPerson/Blueprints/BP_FirstPersonCharacter.BP_FirstPersonCharacter_C|GetCableToWall (Variables|Default|GetFirstPlayerCharacter)) (Math|Transform|InverseTransformLocation (Transformation|GetActorTransform (Variables|Default|GetFirstPlayerCharacter)) (Variables|Default|GetWallHookLocation)))
            ;[1 1 1] Pull Force Character To Wall
            (if (Variables|Default|GetIsPullingToWall?)
              (Default|Drain (Variables|Default|GetFirstPlayerCharacter) 0.5)
              (Physics|AddForce (Variables|/Script/Engine.Character|GetCharacterMovement (Variables|Default|GetFirstPlayerCharacter)) (* (Math|Vector|Normalize (+ (Math|Vector|GetUnitDirection(Vector) (Transformation|GetActorLocation (Variables|Default|GetFirstPlayerCharacter)) (Variables|Default|GetWallHookLocation)) (* (* (Transformation|GetActorRightVector (Variables|Default|GetFirstPlayerCharacter)) (.Y (Math|Vector2D|BreakVector2D (Input|EnhancedActionValues|GetIA_Move)))) 0.7))) 2.5e+05))))
          (:else))))
    (:then_1
      (if (Variables|Default|GetIsGrapplingItem?)
        ;[1 1 1] Setting End Point of the ItemHook
        (bind _itemhook (Variables|Default|GetItemHook)
          (:then
            (Variables|Default|SetItemHookLocation (Transformation|GetActorLocation _itemhook))
            (Variables|/Script/CableComponent.CableComponent|SetEndLocation (Variables|/Game/LemGame/Player/FirstPerson/Blueprints/BP_FirstPersonCharacter.BP_FirstPersonCharacter_C|GetCableToItem (Variables|Default|GetFirstPlayerCharacter)) (Math|Transform|InverseTransformLocation (Transformation|GetActorTransform (Variables|Default|GetFirstPlayerCharacter)) (Variables|Default|GetItemHookLocation)))
            ;[1 1 1] Item Pulling Logic
            (if (Variables|Default|GetIsPullingItem?)
              (Default|Drain (Variables|Default|GetFirstPlayerCharacter) 0.5)
              (Physics|AddForce (Actor|GetComponentbyClass (Variables|/Game/LemGame/Core/GrapplingHook/BP_LightHookFinal.BP_LightHookFinal_C|GetActorToPull (Variables|Default|GetItemHook)) "/Script/Engine.PrimitiveComponent") (* (Math|Vector|Normalize (Math|Vector|GetUnitDirection(Vector) (Transformation|GetActorLocation (Variables|/Game/LemGame/Core/GrapplingHook/BP_LightHookFinal.BP_LightHookFinal_C|GetActorToPull (Variables|Default|GetItemHook))) (.location (Transformation|GetActorTransform (Variables|Default|GetFirstPlayerCharacter))))) (* 5e+05 1.0)) "None" false)))
          (:else))))))