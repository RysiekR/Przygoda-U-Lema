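; BP_EnergyTap is an energy source actor that charges eligible actors while they stand inside its box volume.
; Box overlap events add and remove actors implementing BPI_EnergyDrain in a unique tracking list.
; Tick sends a fixed Charge message to every listed actor each frame, without delta-time scaling, so the charge rate follows frame rate.
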(event OnComponentBeginOverlap(Box)
  (params (OverlappedComponent :type Primitive%20Component%20Object%20Reference) (OtherActor :type Actor%20Object%20Reference) (OtherComp :type Primitive%20Component%20Object%20Reference) (OtherBodyIndex :type Integer) (bFromSweep :type Boolean) (SweepResult :type Hit%20Result%20Structure%20%28by%20ref%29))
  (if (Utilities|DoesObjectImplementInterface OtherActor "/Game/LemGame/Core/Energy/BPI_EnergyDrain.BPI_EnergyDrain_C")
    (Utilities|Array|AddUnique (Variables|Default|GetActorsToDrain) OtherActor)))

(event OnComponentEndOverlap(Box)
  (params (OverlappedComponent :type Primitive%20Component%20Object%20Reference) (OtherActor :type Actor%20Object%20Reference) (OtherComp :type Primitive%20Component%20Object%20Reference) (OtherBodyIndex :type Integer))
  (bind _actorstodrain (Variables|Default|GetActorsToDrain))
  (if (Utilities|DoesObjectImplementInterface OtherActor "/Game/LemGame/Core/Energy/BPI_EnergyDrain.BPI_EnergyDrain_C")
    (if (Utilities|Array|ContainsItem _actorstodrain OtherActor)
      (Utilities|Array|RemoveItem _actorstodrain OtherActor))))

(event EventTick
  (params (DeltaSeconds :type Float%20%28single-precision%29))
  (for _array_element (Variables|Default|GetActorsToDrain)
    (Class|BPIEnergyDrain|Charge(Message) _array_element 1.0)))

(fn ConstructionScript)