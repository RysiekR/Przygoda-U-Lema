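; AC_EnergyBase is an energy component that tracks a clamped energy amount between zero and a maximum.
; On BeginPlay it binds its own DrainEnergy and ChargeEnergy dispatchers to handlers that subtract or add energy.
; The handlers fire FullDischarge when energy reaches zero and FullCharge when it reaches the maximum.
; A helper function returns the current energy as a fraction of the maximum.
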(event Custom|DrainEnergy_Event
  (params (AmountToDrain :type Float%20%28double-precision%29))
  (bind _output_get (Variables|Default|SetEnergyAmount (Math|Float|Clamp(Float) (- (Variables|Default|GetEnergyAmount) AmountToDrain) 0.0 (Variables|Default|GetMaxEnergy))))
  (if (<= _output_get 0.0)
    (Default|CallFullDischarge)))

(event Custom|ChargeEnergy_Event
  (params (EnergyToAdd :type Float%20%28double-precision%29))
  (bind _output_get (Variables|Default|SetEnergyAmount (Math|Float|Clamp(Float) (+ EnergyToAdd (Variables|Default|GetEnergyAmount)) 0.0 (Variables|Default|GetMaxEnergy))))
  (if (>= _output_get (Variables|Default|GetMaxEnergy))
    (Default|CallFullCharge)))

(event EventBeginPlay
  (EventDispatchers|BindEventtoDrainEnergy (delegate Custom|DrainEnergy_Event))
  (EventDispatchers|BindEventtoChargeEnergy (delegate Custom|ChargeEnergy_Event)))

(fn EnergyProcentage
  (return (/ (Variables|Default|GetEnergyAmount) (Variables|Default|GetMaxEnergy))))