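; BP_EnergyTrap is an energy trap volume that drains actors inside its Box that implement BPI_EnergyDrain.
; Box overlaps add and remove those actors from a ToDrain list, and DrainEachInside calls Drain on the list with a zero argument.
; A looping timer created paused at BeginPlay resumes when such an actor enters and pauses again once the list empties, avoiding Tick.
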(event OnComponentBeginOverlap(Box)
  (params (OverlappedComponent :type Primitive%20Component%20Object%20Reference) (OtherActor :type Actor%20Object%20Reference) (OtherComp :type Primitive%20Component%20Object%20Reference) (OtherBodyIndex :type Integer) (bFromSweep :type Boolean) (SweepResult :type Hit%20Result%20Structure%20%28by%20ref%29))
  (if (Utilities|DoesObjectImplementInterface OtherActor "/Game/LemGame/Core/Energy/BPI_EnergyDrain.BPI_EnergyDrain_C")
    (bind _asbpi_energy_drain (Utilities|Casting|CastToBPI_EnergyDrain OtherActor))
    (Utilities|Array|AddUnique (Variables|Default|GetToDrain) _asbpi_energy_drain)
    (Utilities|Time|UnpauseTimerbyHandle (Variables|Default|GetHandlerForDrainEvent))))

(event OnComponentEndOverlap(Box)
  (params (OverlappedComponent :type Primitive%20Component%20Object%20Reference) (OtherActor :type Actor%20Object%20Reference) (OtherComp :type Primitive%20Component%20Object%20Reference) (OtherBodyIndex :type Integer))
  (if (Utilities|DoesObjectImplementInterface OtherActor "/Game/LemGame/Core/Energy/BPI_EnergyDrain.BPI_EnergyDrain_C")
    (bind _asbpi_energy_drain (Utilities|Casting|CastToBPI_EnergyDrain OtherActor))
    (Utilities|Array|RemoveItem (Variables|Default|GetToDrain) _asbpi_energy_drain)
    (if (Utilities|Array|IsEmpty (Variables|Default|GetToDrain))
      (Utilities|Time|PauseTimerbyHandle (Variables|Default|GetHandlerForDrainEvent)))))

(event Custom|DrainEachInside
  (Default|Drain (Variables|Default|GetToDrain) 0.0))

(event EventBeginPlay
  (bind _returnvalue (Utilities|Time|SetTimerbyEvent (EventDispatchers|CreateEvent :!event Custom|DrainEachInside) 0.1 true))
  (bind _output_get (Variables|Default|SetHandlerForDrainEvent _returnvalue))
  (Utilities|Time|PauseTimerbyHandle _output_get))

(fn ConstructionScript)