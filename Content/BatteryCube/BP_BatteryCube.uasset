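; BP_BatteryCube is a battery actor that drains energy from a player inside its box trigger and charges itself until full.
; Box overlaps track the tagged player and show or hide an EnergyCable attached to them, while Tick transfers a fixed amount each frame.
; Drain and Charge events pass through the Energy component, then scale the point light's intensity to the charge level.
; The full-discharge handler is empty.
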(event OnComponentBeginOverlap(Box)
  (params (OverlappedComponent :type Primitive%20Component%20Object%20Reference) (OtherActor :type Actor%20Object%20Reference) (OtherComp :type Primitive%20Component%20Object%20Reference) (OtherBodyIndex :type Integer) (bFromSweep :type Boolean) (SweepResult :type Hit%20Result%20Structure%20%28by%20ref%29))
  (if (Actor|ActorHasTag OtherActor "Player")
    (bind _output_get (Variables|Default|SetPlayer OtherActor))
    (Variables|Default|SetHasPlayer true)
    (Class|CableComponent|SetAttachEndto (Variables|Default|GetEnergyCable) _output_get "CableBatteryPoint" "None")
    (Rendering|SetVisibility (Variables|Default|GetEnergyCable) true false)))

(event OnComponentEndOverlap(Box)
  (params (OverlappedComponent :type Primitive%20Component%20Object%20Reference) (OtherActor :type Actor%20Object%20Reference) (OtherComp :type Primitive%20Component%20Object%20Reference) (OtherBodyIndex :type Integer))
  (if (Actor|ActorHasTag OtherActor "Player")
    (Rendering|SetVisibility (Variables|Default|GetEnergyCable) false false)
    (Class|CableComponent|SetAttachEndto (Variables|Default|GetEnergyCable) self "None" "None")
    (Variables|Default|SetPlayer 0)
    (Variables|Default|SetHasPlayer false)))

(event Custom|FullDischarge_Event)

(event Custom|UpdateBattery
  (bind _output_get (Variables|Default|SetLightLevel (* (Default|EnergyProcentage (Variables|Default|GetEnergy)) (Variables|Default|GetMaxLight))))
  (Rendering|Components|Light|SetIntensity (Variables|Default|GetPointLight) _output_get))

(event EventBeginPlay
  (EventDispatchers|BindEventtoFullDischarge (Variables|Default|GetEnergy) (EventDispatchers|CreateEvent :!event Custom|FullDischarge_Event))
  (CallFunction|UpdateBattery))

(event EventDrain
  (params (Amount :type Float%20%28double-precision%29))
  (Default|CallDrainEnergy (Variables|Default|GetEnergy) Amount)
  (CallFunction|UpdateBattery))

(event EventCharge
  (params (Amount :type Float%20%28double-precision%29))
  (Default|CallChargeEnergy (Variables|Default|GetEnergy) Amount)
  (CallFunction|UpdateBattery))

(event EventTick
  (params (DeltaSeconds :type Float%20%28single-precision%29))
  (bind _energydrainfromplayer (Variables|Default|GetEnergyDrainFromPlayer))
  (if (and (Variables|Default|GetHasPlayer) (!= (Default|EnergyProcentage (Variables|Default|GetEnergy)) 1.0))
    (Class|BPIEnergyDrain|Drain(Message) (Variables|Default|GetPlayer) _energydrainfromplayer)
    (CallFunction|Charge _energydrainfromplayer)))

(fn ConstructionScript)